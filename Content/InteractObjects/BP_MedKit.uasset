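; Medkit pickup that heals a BP_Character on overlap and expires 15 seconds after spawning.
; It acts only if health is below maximum, playing a sound, adding HealAmount truncated and clamped to max, then destroying itself.
; It updates the character's health UI and low-health effect directly, passing a hardcoded 100 maximum to the health update.
; Tick spins the mesh by a fixed per-frame rotation, independent of delta time.
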(event `self.ReceiveBeginPlay`
  (`self.SetLifeSpan` 15.0))

(event `self.ReceiveActorBeginOverlap`
  (params (OtherActor :type "Actor Object Reference"))
  (bind _as_bp_character (`self.As BP Character`))
  (bind _as_bp_character_2 (`self.As BP Character`))
  (bind _as_bp_character_3 (`self.As BP Character`))
  (bind _as_bp_character_4 (`self.As BP Character`))
  (bind _asbp_character (cast `/Game/FPSTest/Core/BP_Character` OtherActor))
  (set `self.As BP Character` _asbp_character)
  (if (< (`/Game/FPSTest/Core/BP_Character.CurrentHealth` _as_bp_character) (`/Game/FPSTest/Core/BP_Character.MaxHealth` _as_bp_character))
    (`GameplayStatics.PlaySound2D` (`self.PickUpSound`) 1.0 1.0 0.0 null null)
    (bind _output_get (set `/Game/FPSTest/Core/BP_Character.CurrentHealth` (`KismetMathLibrary.Conv_IntToDouble` (`KismetMathLibrary.Clamp` (`KismetMathLibrary.FTrunc` (+ (`/Game/FPSTest/Core/BP_Character.CurrentHealth` _as_bp_character_2) (`self.HealAmount`))) 0 (`KismetMathLibrary.FTrunc` (`/Game/FPSTest/Core/BP_Character.MaxHealth` _as_bp_character_2)))) _as_bp_character_3))
    (`/Game/FPSTest/Core/WBP_PlayerUI.UpdateHealth` (`/Game/FPSTest/Core/BP_Character.HealthUIRef` _as_bp_character_3) _output_get 100.0)
    (`/Game/FPSTest/Core/WBP_PlayerUI.UpdateLowHealthEffect` (`/Game/FPSTest/Core/BP_Character.HealthUIRef` (`self.As BP Character`)) (`/Game/FPSTest/Core/BP_Character.CurrentHealth` _as_bp_character_4) (`/Game/FPSTest/Core/BP_Character.MaxHealth` _as_bp_character_4))
    (`self.K2_DestroyActor`)))

(event `self.ReceiveTick`
  (params (DeltaSeconds :type "Float (single-precision)"))
  (`SceneComponent.K2_AddLocalRotation` (`self.Fallout_Medkit`) (struct :`Roll` 1.0) false false))

(fn `UserConstructionScript`)