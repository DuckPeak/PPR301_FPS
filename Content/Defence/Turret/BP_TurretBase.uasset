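; BP_TurretBase is a base turret actor for the defence system, with health, damage and repair handling.
; A hidden health bar widget appears and updates on damage, while Tick rotates it toward the player pawn.
; Repair restores full health and updates the bar, but NeedsRepair always returns false.
; At zero health the turret gathers Enemy-tagged actors in an empty loop, then destroys itself.
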(event `self.ReceiveBeginPlay`
  (bind _aswbp_health_bar (cast `/Game/Build_Objects/WBP_HealthBar` (`WidgetComponent.GetUserWidgetObject` (`self.HealthBar`))))
  (`Widget.SetVisibility` _aswbp_health_bar "Hidden"))

(event `self.ReceiveTick`
  (params (DeltaSeconds :type "Float (single-precision)"))
  (`SceneComponent.K2_SetWorldRotation` (`self.HealthBar`) (`KismetMathLibrary.FindLookAtRotation` (`self.K2_GetActorLocation`) (`self.K2_GetActorLocation` (`GameplayStatics.GetPlayerPawn` 0))) false false))

(event `self.Repair`
  (set `self.CurrentHealth` (`self.MaxHealth`))
  (bind _aswbp_health_bar (cast `/Game/Build_Objects/WBP_HealthBar` (`WidgetComponent.GetUserWidgetObject` (`self.HealthBar`))))
  (`/Game/Build_Objects/WBP_HealthBar.SetHealthPercent` _aswbp_health_bar (/ (`self.CurrentHealth`) (`self.MaxHealth`))))

(event `self.ReceiveAnyDamage`
  (params (Damage :type "Float (single-precision)") (DamageType :type "DamageType Object Reference") (InstigatedBy :type "Controller Object Reference") (DamageCauser :type "Actor Object Reference"))
  (bind _output_get (set `self.CurrentHealth` (- (`self.CurrentHealth`) Damage)))
  (bind _aswbp_health_bar (cast `/Game/Build_Objects/WBP_HealthBar` (`WidgetComponent.GetUserWidgetObject` (`self.HealthBar`))))
  (`Widget.SetVisibility` _aswbp_health_bar "Visible")
  (`/Game/Build_Objects/WBP_HealthBar.SetHealthPercent` _aswbp_health_bar (/ _output_get (`self.MaxHealth`)))
  (if (<= _output_get 0.0)
    (bind _outactors (`GameplayStatics.GetAllActorsWithTag` "Enemy"))
    (for _ _outactors
      _)
    (`self.K2_DestroyActor`)))

(fn `NeedsRepair`
  (returns (ReturnValue :type Boolean))
  (return false))

(fn `UserConstructionScript`)