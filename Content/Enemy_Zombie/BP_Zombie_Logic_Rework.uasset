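; Zombie enemy AI that advances on the DefencePoint power station, diverting to Defence-tagged obstacles ahead or a player within aggro range.
; An event-driven state loop uses sphere traces to pick targets, AIMoveTo to approach, and montage-notify traces to deal damage, with delayed recovery.
; Death plays sound, rolls health and ammo drops, notifies the wave manager and ragdolls before destroying.
; Older patrol and detection logic remains as disconnected leftovers.
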(event `self.ReceiveBeginPlay`
  ; Setup
  (bind _outactors (`GameplayStatics.GetAllActorsOfClass` "/Game/FPSTest/Core/DefencePoint.DefencePoint_C"))
  (set `self.DefencePointRef` (`|GetArrayItem` _outactors))
  (`self.UpdateZombieBehaviour`))

(event `UpdateZombieBehaviour`
  (bind _returnvalue (`self.K2_GetActorLocation`))
  ; UpdateBehaviour
  (if (not (or (`|EnumEquality` (`self.ZombieState`) "NewEnumerator3") (`|EnumEquality` (`self.ZombieState`) "NewEnumerator2") (`|EnumEquality` (`self.ZombieState`) "NewEnumerator4") (== (`self.bIsAttacking`) true) (!= (`self.canAttack`) true)))
    (set `self.FoundDefence` false)
    (if (not (`self.IsDead`))
      (bind (_outhits _returnvalue_2) (`KismetSystemLibrary.SphereTraceMultiForObjects` _returnvalue (+ _returnvalue (* (`KismetMathLibrary.GetForwardVector` (`self.K2_GetActorRotation`)) 250)) 500.0 (`|MakeArray` "ObjectTypeQuery2" "ObjectTypeQuery1" :!type "EObjectTypeQuery Enum")))
      (for _array_element _outhits
        (if _returnvalue_2
          (bind (_bblockinghit _binitialoverlap _time _distance _location _impactpoint _normal _impactnormal _physmat _hitactor) (`GameplayStatics.BreakHitResult` _array_element))
          (if (`self.ActorHasTag` _hitactor "Defence")
            (set `self.FoundDefence` true)
            (set `self.CurrentDefenceTarget` _hitactor)
            (set `self.ZombieState` "NewEnumerator3")
            (`self.AttackCurrentDefence`))))
      (if (not (`self.FoundDefence`))
        (`self.CheckPlayerAggro`)))))

(event `AttackCurrentDefence`
  (bind _returnvalue (`self.K2_GetActorLocation`))
  ; AttackCurrentDefenceTarget
  (if (`KismetSystemLibrary.IsValid` (`self.CurrentDefenceTarget`))
    (`|AIMoveTo` self (0.0 0.0 0.0) (`self.CurrentDefenceTarget`) 150.0
      (:`OnSuccess`
        (if (`self.bIsAttacking`)
          _
          (elif (`self.canAttack`)
            (set `self.bIsAttacking` true)
            (set `self.canAttack` false)
            (`|PlayMontage` (`self.Mesh`) "/Game/ZombieAnimationPack/Animations/Mannequin_UE4/anim_Attack_D_Montage.anim_Attack_D_Montage"
              (:`OnNotifyBegin`
                (bind (_outhit _returnvalue_2) (`KismetSystemLibrary.SphereTraceSingleForObjects` :`Start` _returnvalue :`End` (+ _returnvalue (* (`KismetMathLibrary.GetForwardVector` (`self.K2_GetActorRotation`)) 250)) :`Radius` 120.0 :`ObjectTypes` (`|MakeArray` "ObjectTypeQuery2" :!type "EObjectTypeQuery Enum") :`DrawDebugType` "ForDuration"))
                (if _returnvalue_2
                  (bind (_bblockinghit _binitialoverlap _time _distance _location _impactpoint _normal _impactnormal _physmat _hitactor) (`GameplayStatics.BreakHitResult` _outhit))
                  (if (`self.ActorHasTag` _hitactor "Defence")
                    (`GameplayStatics.ApplyDamage` _hitactor 10.0)
                    (`KismetSystemLibrary.Delay` 2.0)
                    (set `self.canAttack` true)
                    (set `self.bIsAttacking` false)
                    (set `self.ZombieState` "NewEnumerator0")
                    (`self.UpdateZombieBehaviour`)))))
            (else
              (`KismetSystemLibrary.Delay` 0.2)
              (`self.AttackCurrentDefence`)))))
      (:`OnFail`
        (set `self.CurrentDefenceTarget` null :!label _label)
        (set `self.canAttack` true)
        (set `self.bIsAttacking` false)
        (set `self.ZombieState` "NewEnumerator0")
        (`self.MoveToPowerStation`)))
    (else
      (goto _label))))

(event `Patrol`
  ; Old AI
  ;; Attack defence point (Used to be patrol)
)

(event `AttackPowerStation`
  (bind _returnvalue (`self.K2_GetActorLocation`))
  ; AttackMainPoint
  (bind _outactors (`GameplayStatics.GetAllActorsOfClass` "BP_Zombie_Logic_Rework_C"))
  (`self.K2_SetActorRotation` (`KismetMathLibrary.MakeRotator` 0.0 0.0 (.yaw (`KismetMathLibrary.FindLookAtRotation` (`self.K2_GetActorLocation`) (`self.K2_GetActorLocation` (`self.DefencePointRef`))))))
  (if (`self.canAttack`)
    (set `self.canAttack` false)
    (`|PlayMontage` (`self.Mesh`) "/Game/ZombieAnimationPack/Animations/Mannequin_UE4/anim_Attack_D_Montage.anim_Attack_D_Montage"
      (:`OnInterrupted`
        (`KismetSystemLibrary.Delay` 2.0)
        (set `self.canAttack` true)
        (`self.UpdateZombieBehaviour`))
      (:`OnNotifyBegin`
        (bind (_outhit _returnvalue_2) (`KismetSystemLibrary.SphereTraceSingleForObjects` _returnvalue (+ _returnvalue (* (`KismetMathLibrary.GetForwardVector` (`self.K2_GetActorRotation`)) 250)) 120.0 (`|MakeArray` "ObjectTypeQuery2" :!type "EObjectTypeQuery Enum") false _outactors "ForDuration"))
        (if _returnvalue_2
          (bind (_bblockinghit _binitialoverlap _time _distance _location _impactpoint _normal _impactnormal _physmat _hitactor _hitcomponent) (`GameplayStatics.BreakHitResult` _outhit))
          (if (`ActorComponent.ComponentHasTag` _hitcomponent "DefencePoint")
            (`GameplayStatics.ApplyDamage` _hitactor 10.0)
            (`KismetSystemLibrary.Delay` 2.0)
            (set `self.canAttack` true)
            (set `self.bIsAttacking` false)
            (set `self.ZombieState` "NewEnumerator0")
            (`self.UpdateZombieBehaviour`))
          (else
            (set `self.canAttack` true)
            (`KismetSystemLibrary.Delay` 2.0)
            (set `self.ZombieState` "NewEnumerator0")
            (`self.MoveToPowerStation`)))))))

(event `MoveToPowerStation`
  ; MoveToMainDefence
  (`|ExecutionSequence`
    (:`then_0`
      (`|AIMoveTo` self (0.0 0.0 0.0) (`self.DefencePointRef`) 200.0
        (:`OnSuccess`
          (set `self.ZombieState` "NewEnumerator4")
          (`self.AttackPowerStation`))
        (:`OnFail`
          (`KismetSystemLibrary.Delay` 0.2 :!label _label_2)
          (`self.UpdateZombieBehaviour`))))
    (:`then_1`
      (goto _label_2))))

(event `CheckPlayerAggro`
  ; FindPlayerInRange
  (if (<= (`self.GetDistanceTo` (`GameplayStatics.GetPlayerCharacter` 0) self) (`self.AggroRange`))
    (set `self.PlayerTarget` (`GameplayStatics.GetPlayerCharacter` 0))
    (set `self.ZombieState` "NewEnumerator1")
    (`self.ChasePlayer`)
    (else
      (set `self.ZombieState` "NewEnumerator0")
      (`self.MoveToPowerStation`))))

(event `ChasePlayer`
  ; ChasePlayer
  (`|AIMoveTo` self (0.0 0.0 0.0) (`self.PlayerTarget`) 120.0
    (:`OnSuccess`
      (set `self.ZombieState` "NewEnumerator2")
      (`self.AttackPlayer`))
    (:`OnFail`
      (`KismetSystemLibrary.Delay` 0.2)
      (`self.UpdateZombieBehaviour`))))

(event `AttackPlayer`
  (bind _returnvalue (`self.K2_GetActorLocation`))
  ; AttackThePlayer
  (if (`self.bIsAttacking`)
    _
    (elif (`self.canAttack`)
      (set `self.bIsAttacking` true)
      (set `self.canAttack` false)
      (`|PlayMontage` (`self.Mesh`) "/Game/ZombieAnimationPack/Animations/Mannequin_UE4/anim_Attack_D_Montage.anim_Attack_D_Montage"
        (:`OnCompleted`
          (`self.Recovery` :!label _label_3))
        (:`OnInterrupted`
          (goto _label_3))
        (:`OnNotifyBegin`
          (bind _outactors (`GameplayStatics.GetAllActorsOfClass` "BP_Zombie_Logic_Rework_C"))
          (bind (_outhit _returnvalue_2) (`KismetSystemLibrary.SphereTraceSingleForObjects` _returnvalue (+ _returnvalue (* (`KismetMathLibrary.GetForwardVector` (`self.K2_GetActorRotation`)) 250)) 120.0 (`|MakeArray` "ObjectTypeQuery3" :!type "EObjectTypeQuery Enum") false _outactors "ForDuration"))
          (if _returnvalue_2
            (bind (_bblockinghit _binitialoverlap _time _distance _location _impactpoint _normal _impactnormal _physmat _hitactor) (`GameplayStatics.BreakHitResult` _outhit))
            (if (== _hitactor (`self.PlayerTarget`))
              (`GameplayStatics.ApplyDamage` _hitactor 10.0)
              (`KismetSystemLibrary.Delay` 2.0)
              (set `self.canAttack` true)
              (set `self.bIsAttacking` false)
              (set `self.ZombieState` "NewEnumerator2")
              (`self.CheckPlayerAggro`)
              (else
                (`self.Recovery`)))
            (else
              (set `self.canAttack` true)
              (set `self.bIsAttacking` false)
              (set `self.ZombieState` "NewEnumerator2")
              (`self.CheckPlayerAggro`))))))))

(event `ChaseTarget`
  (params (TargetActor :type "Actor Object Reference"))
  ; Old AI
  ;; Attack player when spotted
)

(event `FindBlockingDefence`)

(event `ClearDefenceTarget`)

(event `self.ReceiveAnyDamage`
  (params (Damage :type "Float (single-precision)") (DamageType :type "DamageType Object Reference") (InstigatedBy :type "Controller Object Reference") (DamageCauser :type "Actor Object Reference"))
  ; HP logic
  (`GameplayStatics.PlaySoundAtLocation` (`|GetArrayItem` (`self.HitSounds`) (`KismetMathLibrary.RandomIntegerInRange` 0 3)) (`self.K2_GetActorLocation`) (struct) 1.0 (`KismetMathLibrary.RandomFloatInRange` 0.9 1.1) 0.0 "/Game/FPSTest/Core/SA_ZombieAttack.SA_ZombieAttack" null null null)
  (bind _output_get (set `self.CurrentHealth` (- (`self.CurrentHealth`) Damage)))
  (`KismetSystemLibrary.PrintString` (`KismetStringLibrary.Conv_DoubleToString` _output_get))
  (if (and (<= (`self.CurrentHealth`) 0.0) (not (`self.IsDead`)))
    (`self.Death`)))

(event `Death`
  (bind _wavemanagerref (`self.WaveManagerRef`))
  ; Death Logic
  (`GameplayStatics.PlaySoundAtLocation` (`|GetArrayItem` (`self.DieSounds`) (`KismetMathLibrary.RandomIntegerInRange` 0 3)) (`self.K2_GetActorLocation`) (struct) 1.0 (`KismetMathLibrary.RandomFloatInRange` 0.9 1.1) 0.0 "/Game/FPSTest/Core/SA_ZombieAttack.SA_ZombieAttack" null null null)
  (set `self.IsDead` true)
  (if (<= (`KismetMathLibrary.RandomFloatInRange` 0.0 1.0) (`self.HealthDropChance`))
    (`|SpawnActorFromClass` (`self.HealthDropClass`) (`KismetMathLibrary.Conv_VectorToTransform` (`self.K2_GetActorLocation`)) "Undefined" "MultiplyWithRoot" null null))
  (if (<= (`KismetMathLibrary.RandomFloatInRange` 0.0 1.0) (`self.AmmoDropChance`))
    (`|SpawnActorFromClass` (`self.AmmoDropClass`) (`KismetMathLibrary.Conv_VectorToTransform` (`self.K2_GetActorLocation`)) "Undefined" "MultiplyWithRoot" null null))
  (`|ExecutionSequence`
    (:`then_0`
      (`/Engine/EditorBlueprintResources/StandardMacros.IsValid` _wavemanagerref
        (:`Is Valid`
          (`WaveManager.OnEnemyKilled` _wavemanagerref))))
    (:`then_1`
      (`CharacterMovementComponent.DisableMovement` (`self.CharacterMovement`))
      (`PrimitiveComponent.SetCollisionEnabled` (`self.CapsuleComponent`) "NoCollision")
      (`PrimitiveComponent.SetCollisionProfileName` (`self.Mesh`) "Ragdoll" true)
      (`SkeletalMeshComponent.SetAllBodiesSimulatePhysics` (`self.Mesh`) true)
      (`PrimitiveComponent.WakeAllRigidBodies` (`self.Mesh`))
      (`SkeletalMeshComponent.SetPhysicsBlendWeight` (`self.Mesh`) 1.0)
      (`KismetSystemLibrary.Delay` 5.0)
      (`self.K2_DestroyActor`))))

(event `FindNextDefenceTarget`
  ; Old AI
  ;; Target reset function
)

(event `Recovery`
  (`KismetSystemLibrary.Delay` 2.0)
  (set `self.canAttack` true)
  (set `self.bIsAttacking` false)
  (set `self.ZombieState` "NewEnumerator1")
  (`self.CheckPlayerAggro`))

(fn `UserConstructionScript`)