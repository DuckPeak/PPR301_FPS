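; Wave-based zombie enemy that walks to the DefencePoint, attacks nearby defences on the way and chases pawns it sees.
; AI MoveTo drives movement, a detection sphere picks Defence-tagged targets, and pawn sensing triggers the chase.
; Attack montage notifies run forward sphere traces to apply damage.
; On death it randomly drops health or ammo, notifies the wave manager and ragdolls before being destroyed.
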(event `self.ReceiveBeginPlay`
  ; Setup
  (bind _outactors (`GameplayStatics.GetAllActorsOfClass` "/Game/FPSTest/Core/DefencePoint.DefencePoint_C"))
  (set `self.DefencePointRef` (`|GetArrayItem` _outactors))
  (`self.Patrol`))

(event `self.PawnSensing.OnSeePawn`
  (params (Pawn :type "Pawn Object Reference"))
  ; Setup
  (if (not (`self.IsDead`))
    (`self.ChaseTarget` Pawn)))

(event `Patrol`
  (bind _returnvalue (`self.K2_GetActorLocation`))
  (bind _returnvalue_2 (`self.K2_GetActorLocation`))
  (bind _currentdefencetarget (`self.CurrentDefenceTarget`))
  ; Attack defence point (Used to be patrol)
  (if (not (`self.IsDead`))
    (`|AIMoveTo` self (`self.K2_GetActorLocation` (select `bool` (`KismetSystemLibrary.IsValid` _currentdefencetarget) :`false` (`self.DefencePointRef`) :`true` _currentdefencetarget)) null 200.0
      (:`OnSuccess`
        (if (and (`self.canAttack`) (`KismetSystemLibrary.IsValid` (`self.CurrentDefenceTarget`)) (`self.bAttackingDefence`))
          (`GameplayStatics.PlaySoundAtLocation` (`|GetArrayItem` (`self.AttackSounds`) (`KismetMathLibrary.RandomIntegerInRange` 0 3)) (`self.K2_GetActorLocation`) (struct) 1.0 (`KismetMathLibrary.RandomFloatInRange` 0.9 1.1) 0.0 "/Game/FPSTest/Core/SA_ZombieAttack.SA_ZombieAttack" null null null)
          (`|PlayMontage` (`self.Mesh`) "/Game/ZombieAnimationPack/Animations/Mannequin_UE4/anim_Attack_D_Montage.anim_Attack_D_Montage"
            (:`then`
              (set `self.canAttack` false))
            (:`OnCompleted`
              (set `self.canAttack` true :!label _label)
              (`/Engine/EditorBlueprintResources/StandardMacros.IsValid` (`self.CurrentDefenceTarget`)
                (:`Is Valid`
                  (`self.Patrol`))))
            (:`OnBlendOut`
              (`self.Patrol`))
            (:`OnInterrupted`
              (goto _label))
            (:`OnNotifyBegin`
              (`/Engine/EditorBlueprintResources/StandardMacros.IsValid` (`self.CurrentDefenceTarget`)
                (:`Is Valid`
                  (bind _outactors (`GameplayStatics.GetAllActorsOfClass` "BP_Zombie_C"))
                  (bind (_outhit _returnvalue_3) (`KismetSystemLibrary.SphereTraceSingleForObjects` _returnvalue_2 (+ _returnvalue_2 (* (`KismetMathLibrary.GetForwardVector` (`self.K2_GetActorRotation`)) 200.0)) 20.0 (`|MakeArray` "ObjectTypeQuery2" :!type "EObjectTypeQuery Enum") false _outactors "None" true (struct :`R` 1.0 :`A` 1.0) (struct :`G` 1.0 :`A` 1.0) 0.5))
                  (if _returnvalue_3
                    (bind (_bblockinghit _binitialoverlap _time _distance _location _impactpoint _normal _impactnormal _physmat _hitactor) (`GameplayStatics.BreakHitResult` _outhit))
                    (if (`self.ActorHasTag` _hitactor "Defence")
                      (`GameplayStatics.ApplyDamage` _hitactor 10.0))))
                (:`Is Not Valid`
                  (`self.StopAnimMontage` "/Game/ZombieAnimationPack/Animations/Mannequin_UE4/anim_Attack_D_Montage.anim_Attack_D_Montage")
                  (set `self.canAttack` true)
                  (set `self.bAttackingDefence` false)
                  (set `self.CurrentDefenceTarget` null)
                  (`self.Patrol`)))))
          (else
            (`GameplayStatics.PlaySoundAtLocation` (`|GetArrayItem` (`self.AttackSounds`) (`KismetMathLibrary.RandomIntegerInRange` 0 3)) (`self.K2_GetActorLocation`) (struct) 1.0 (`KismetMathLibrary.RandomFloatInRange` 0.9 1.1) 0.0 "/Game/FPSTest/Core/SA_ZombieAttack.SA_ZombieAttack" null null null)
            (`|PlayMontage` (`self.Mesh`) "/Game/ZombieAnimationPack/Animations/Mannequin_UE4/anim_Attack_D_Montage.anim_Attack_D_Montage"
              (:`OnNotifyBegin`
                (bind _outactors_2 (`GameplayStatics.GetAllActorsOfClass` "BP_Zombie_C"))
                (bind (_outhit_2 _returnvalue_4) (`KismetSystemLibrary.SphereTraceSingleForObjects` _returnvalue (+ _returnvalue (* (`KismetMathLibrary.GetForwardVector` (`self.K2_GetActorRotation`)) 200.0)) 20.0 (`|MakeArray` "ObjectTypeQuery2" :!type "EObjectTypeQuery Enum") false _outactors_2 "None" true (struct :`R` 1.0 :`A` 1.0) (struct :`G` 1.0 :`A` 1.0) 0.5))
                (if _returnvalue_4
                  (bind (_bblockinghit_2 _binitialoverlap_2 _time_2 _distance_2 _location_2 _impactpoint_2 _normal_2 _impactnormal_2 _physmat_2 _hitactor_2) (`GameplayStatics.BreakHitResult` _outhit_2))
                  (if (`self.ActorHasTag` _hitactor_2 "DefencePoint")
                    (`GameplayStatics.ApplyDamage` _hitactor_2 10.0)
                    (`KismetSystemLibrary.Delay` 2.0)
                    (`self.Patrol`)
                    (else
                      (`self.Patrol`)))))))))
      (:`OnFail`
        (`self.Patrol`)))))

(event `ChaseTarget`
  (params (TargetActor :type "Actor Object Reference"))
  (bind _returnvalue (`self.K2_GetActorLocation`))
  ; Attack player when spotted
  (if (not (`self.IsDead`))
    (`|AIMoveTo` self (0.0 0.0 0.0) TargetActor 120.0 true
      (:`OnSuccess`
        (if (`self.canAttack`)
          (`GameplayStatics.PlaySoundAtLocation` (`|GetArrayItem` (`self.AttackSounds`) (`KismetMathLibrary.RandomIntegerInRange` 0 3)) (0.0 0.0 0.0) (struct) 1.0 (`KismetMathLibrary.RandomFloatInRange` 0.9 1.1) 0.0 "/Game/FPSTest/Core/SA_ZombieAttack.SA_ZombieAttack" null null null)
          (`|PlayMontage` (`self.Mesh`) "/Game/ZombieAnimationPack/Animations/Mannequin_UE4/anim_Attack_D_Montage.anim_Attack_D_Montage" 2.5
            (:`then`
              (set `self.canAttack` false))
            (:`OnCompleted`
              (set `self.canAttack` true :!label _label_2))
            (:`OnBlendOut`
              (`self.Patrol`))
            (:`OnInterrupted`
              (goto _label_2))
            (:`OnNotifyBegin`
              (bind (_outhit _returnvalue_2) (`KismetSystemLibrary.SphereTraceSingleForObjects` :`Start` _returnvalue :`End` (+ _returnvalue (* (`KismetMathLibrary.GetForwardVector` (`self.K2_GetActorRotation`)) 200.0)) :`Radius` 20.0 :`ObjectTypes` (`|MakeArray` "ObjectTypeQuery3" :!type "EObjectTypeQuery Enum") :`DrawTime` 0.5))
              (if _returnvalue_2
                (`GameplayStatics.ApplyDamage` (`.HitActor` (`GameplayStatics.BreakHitResult` _outhit)) 10.0)))))))))

(event `self.ReceiveAnyDamage`
  (params (Damage :type "Float (single-precision)") (DamageType :type "DamageType Object Reference") (InstigatedBy :type "Controller Object Reference") (DamageCauser :type "Actor Object Reference"))
  ; HP logic
  (`GameplayStatics.PlaySoundAtLocation` (`|GetArrayItem` (`self.HitSounds`) (`KismetMathLibrary.RandomIntegerInRange` 0 3)) (`self.K2_GetActorLocation`) (struct) 1.0 (`KismetMathLibrary.RandomFloatInRange` 0.9 1.1) 0.0 "/Game/FPSTest/Core/SA_ZombieAttack.SA_ZombieAttack" null null null)
  (bind _output_get (set `self.CurrentHealth` (- (`self.CurrentHealth`) Damage)))
  (`KismetSystemLibrary.PrintString` (`KismetStringLibrary.Conv_DoubleToString` _output_get))
  (if (and (<= (`self.CurrentHealth`) 0.0) (not (`self.IsDead`)))
    (`self.Death`)))

(event `Death`
  (bind _wavemanagerref (`self.WaveManagerRef`))
  ; Death Logic
  (`GameplayStatics.PlaySoundAtLocation` (`|GetArrayItem` (`self.DieSounds`) (`KismetMathLibrary.RandomIntegerInRange` 0 3)) (`self.K2_GetActorLocation`) (struct) 1.0 (`KismetMathLibrary.RandomFloatInRange` 0.9 1.1) 0.0 "/Game/FPSTest/Core/SA_ZombieAttack.SA_ZombieAttack" null null null)
  (set `self.IsDead` true)
  (if (<= (`KismetMathLibrary.RandomFloatInRange` 0.0 1.0) (`self.HealthDropChance`))
    (`|SpawnActorFromClass` (`self.HealthDropClass`) (`KismetMathLibrary.Conv_VectorToTransform` (`self.K2_GetActorLocation`)) "Undefined" "MultiplyWithRoot" null null))
  (if (<= (`KismetMathLibrary.RandomFloatInRange` 0.0 1.0) (`self.AmmoDropChance`))
    (`|SpawnActorFromClass` (`self.AmmoDropClass`) (`KismetMathLibrary.Conv_VectorToTransform` (`self.K2_GetActorLocation`)) "Undefined" "MultiplyWithRoot" null null))
  (`|ExecutionSequence`
    (:`then_0`
      (`/Engine/EditorBlueprintResources/StandardMacros.IsValid` _wavemanagerref
        (:`Is Valid`
          (`WaveManager.OnEnemyKilled` _wavemanagerref))))
    (:`then_1`
      (`CharacterMovementComponent.DisableMovement` (`self.CharacterMovement`))
      (`PrimitiveComponent.SetCollisionEnabled` (`self.CapsuleComponent`) "NoCollision")
      (`PrimitiveComponent.SetCollisionProfileName` (`self.Mesh`) "Ragdoll" true)
      (`SkeletalMeshComponent.SetAllBodiesSimulatePhysics` (`self.Mesh`) true)
      (`PrimitiveComponent.WakeAllRigidBodies` (`self.Mesh`))
      (`SkeletalMeshComponent.SetPhysicsBlendWeight` (`self.Mesh`) 1.0)
      (`KismetSystemLibrary.Delay` 5.0)
      (`self.K2_DestroyActor`))))

(event `self.DefenceDetectionSphere.OnComponentBeginOverlap`
  (params (OverlappedComponent :type "PrimitiveComponent Object Reference") (OtherActor :type "Actor Object Reference") (OtherComp :type "PrimitiveComponent Object Reference") (OtherBodyIndex :type Integer) (bFromSweep :type Boolean) (SweepResult :type "HitResult Structure (by ref)"))
  ; Defence Detection
  (if (`self.ActorHasTag` OtherActor "Defence")
    (if (`KismetSystemLibrary.IsValid` (`self.CurrentDefenceTarget`))
      (if (`self.ActorHasTag` (`self.CurrentDefenceTarget`) "DefencePoint")
        (set `self.CurrentDefenceTarget` OtherActor)
        (set `self.bAttackingDefence` true))
      (else
        (set `self.CurrentDefenceTarget` OtherActor)
        (set `self.bAttackingDefence` true)
        (`self.Patrol`)))))

(event `self.DefenceDetectionSphere.OnComponentEndOverlap`
  (params (OverlappedComponent :type "PrimitiveComponent Object Reference") (OtherActor :type "Actor Object Reference") (OtherComp :type "PrimitiveComponent Object Reference") (OtherBodyIndex :type Integer))
  ; Defence Detection
  (if (== OtherActor (`self.CurrentDefenceTarget`))
    (set `self.CurrentDefenceTarget` null)
    (set `self.bAttackingDefence` false)
    (`self.FindNextDefenceTarget`)))

(event `FindNextDefenceTarget`
  ; Target reset function
  (for _array_element (`PrimitiveComponent.GetOverlappingActors` (`self.DefenceDetectionSphere`) null)
    (if (`self.ActorHasTag` _array_element "Defence")
      (set `self.CurrentDefenceTarget` _array_element)
      (set `self.bAttackingDefence` true)
      (set `self.canAttack` true)
      (`self.Patrol`)))
  (set `self.bAttackingDefence` false)
  (set `self.CurrentDefenceTarget` null)
  (`self.Patrol`))

(fn `UserConstructionScript`)