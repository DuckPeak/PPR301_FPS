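; BP_Weapon is a first-person assault rifle actor that handles the cosmetic side of firing and reloading.
; Shoot plays the fire montage on the rifle's skeletal mesh and spawns a BP_Casing at the ejection socket with a short lifespan.
; The casing's IgnoreActorWhenMoving call passes false, so it does not ignore the player character.
; Reload only plays the reload montage; no projectile, damage or ammo logic is present.
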(event `/Game/FPSTest/Core/BPI_Weapon.Shoot`
  (`|PlayMontage` (`self.SK_AssaultRifle`) "/Game/FPSTest/Art/AssaultRifle/Animations/AM_FP_WEP_AssaultRifle_Fire_Montage.AM_FP_WEP_AssaultRifle_Fire_Montage"
    (:`then`
      (bind _returnvalue (`|SpawnActorFromClass` "/Game/FPSTest/Core/BP_Casing.BP_Casing_C" (`SceneComponent.GetSocketTransform` (`self.SK_AssaultRifle`) "SOCKET_Ejection" "RTS_World") "AlwaysSpawn" "MultiplyWithRoot" null null))
      (`self.SetLifeSpan` _returnvalue 5.0)
      (`PrimitiveComponent.IgnoreActorWhenMoving` (`/Game/FPSTest/Core/BP_Casing.Casing mesh` _returnvalue) (`GameplayStatics.GetPlayerCharacter` 0) false))))

(event `/Game/FPSTest/Core/BPI_Weapon.Reload`
  (`|PlayMontage` (`self.SK_AssaultRifle`) "/Game/FPSTest/Art/AssaultRifle/Animations/AM_A_FP_WP_AssaultRifle_Reload.AM_A_FP_WP_AssaultRifle_Reload"))

(fn `UserConstructionScript`)