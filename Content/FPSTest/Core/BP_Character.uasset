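; BP_Character is the first-person player character, handling movement, weapons, health and the end screen on death.
; Enhanced Input drives walking, timeline-based sprint FOV and crouch capsule height, aiming, holstering and reloading from reserve ammo.
; Inventory weapons spawn attached to the arms, and held fire loops montage, BP_Bullet spawn and delay.
; A per-tick camera trace blocks shooting near walls, and damage updates the health widget.
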(event `self.ReceiveBeginPlay`
  (`EnhancedInputSubsystemInterface.AddMappingContext` (pcsubsystem `EnhancedInputLocalPlayerSubsystem` (`GameplayStatics.GetPlayerController` 0)) "/Game/FPSTest/Data/IMC_FPS.IMC_FPS" 0 (struct))
  ; Create UI
  (`self.SpawnInventory`)
  (bind _returnvalue (`|CreateWidget` "/Game/FPSTest/Core/WBP_PlayerUI.WBP_PlayerUI_C" (`GameplayStatics.GetPlayerController` 0)))
  (set `self.HealthUIRef` _returnvalue)
  (`UserWidget.AddToViewport` _returnvalue 0)
  (`self.HolsterToggle`))

(event `EnhancedInput|/Game/FPSTest/Data/IA_Movement`
  (params (ActionValue :type "Vector2D Structure") (ElapsedSeconds :type "Float (double-precision)") (TriggeredSeconds :type "Float (double-precision)") (InputAction :type "InputAction Object Reference" :default "/Game/FPSTest/Data/IA_Movement.IA_Movement"))
  (bind (_x _y) (`KismetMathLibrary.BreakVector2D` (`self.MoveInput`)))
  ; Camera/Movement
  (:`Triggered`
    (set `self.MoveInput` ActionValue :!label _label)
    (`self.AddMovementInput` (* _y (`self.GetActorForwardVector`)))
    (`self.AddMovementInput` (* _x (`self.GetActorRightVector`))))
  (:`Completed`
    (goto _label)))

(event `EnhancedInput|/Game/FPSTest/Data/IA_Camera`
  (params (ActionValue :type "Vector2D Structure") (ElapsedSeconds :type "Float (double-precision)") (TriggeredSeconds :type "Float (double-precision)") (InputAction :type "InputAction Object Reference" :default "/Game/FPSTest/Data/IA_Camera.IA_Camera"))
  (bind (_x _y) (`KismetMathLibrary.BreakVector2D` (`self.MouseInput`)))
  ; Camera/Movement
  (:`Triggered`
    (set `self.MouseInput` ActionValue :!label _label_2)
    (`self.AddControllerYawInput` _x)
    (`self.AddControllerPitchInput` (* _y -1.0)))
  (:`Completed`
    (goto _label_2)))

(event `EnhancedInput|/Game/FPSTest/Data/IA_Run`
  (params (ActionValue :type Boolean) (ElapsedSeconds :type "Float (double-precision)") (TriggeredSeconds :type "Float (double-precision)") (InputAction :type "InputAction Object Reference" :default "/Game/FPSTest/Data/IA_Run.IA_Run"))
  ; Running/FOV
  (:`Triggered`
    (if (`self.bCanRun`)
      (if (`NavMovementInterface.IsFalling` (`self.CharacterMovement`))
        _
        (elif (not (`self.bCrouching`))
          (set `self.bRunning` true)
          (set `CharacterMovementComponent.MaxWalkSpeed` (`self.RunningSpeed`) (`self.CharacterMovement`))
          (if (> (`KismetMathLibrary.VSize` (`self.GetVelocity`)) 0.0)
            (bind (_direction _fov) (`Timeline|Timeline` :!label _label_3)
              (:`Update`
                (`CameraComponent.SetFieldOfView` (`self.Camera`) _fov)))
            (else
              (goto _label_3 :!via `Reverse`)))))))
  (:`Completed`
    (`self.Stop Running`)))

(event `Stop Running`
  ; Running/FOV
  (set `self.bRunning` false)
  (set `CharacterMovementComponent.MaxWalkSpeed` 600.0 (`self.CharacterMovement`))
  (goto _label_3 :!via `Reverse`))

(event `EnhancedInput|/Game/FPSTest/Data/IA_Jump`
  (params (ActionValue :type Boolean) (ElapsedSeconds :type "Float (double-precision)") (TriggeredSeconds :type "Float (double-precision)") (InputAction :type "InputAction Object Reference" :default "/Game/FPSTest/Data/IA_Jump.IA_Jump"))
  ; Running/FOV
  (:`Triggered`
    (`self.Jump`)
    (`self.Stop Running`))
  (:`Completed`
    (`self.StopJumping`)))

(event `EnhancedInput|/Game/FPSTest/Data/IA_Crouch`
  (params (ActionValue :type Boolean) (ElapsedSeconds :type "Float (double-precision)") (TriggeredSeconds :type "Float (double-precision)") (InputAction :type "InputAction Object Reference" :default "/Game/FPSTest/Data/IA_Crouch.IA_Crouch"))
  ; Crouching
  (:`Triggered`
    (`/Engine/EditorBlueprintResources/StandardMacros.DoOnce` false :!label _label_4
      (:`Completed`
        (if (`self.bHoldCrouch`)
          (`self.CustomCrouch`)
          (else
            (`/Engine/EditorBlueprintResources/StandardMacros.FlipFlop`
              (:`A`
                (`self.CustomCrouch`))
              (:`B`
                (`self.CustomUnCrouch`))))))))
  (:`Completed`
    (`|ExecutionSequence`
      (:`then_0`
        (if (`self.bHoldCrouch`)
          (`self.CustomUnCrouch`)))
      (:`then_1`
        (goto _label_4 :!via `Reset`)))))

(event `CustomCrouch`
  ; Crouching
  (set `self.bCrouching` true)
  (`self.Stop Running`)
  (set `CharacterMovementComponent.MaxWalkSpeed` 400.0 (`self.CharacterMovement`))
  (bind (_direction _half_height) (`Timeline|CrouchTimeline` :!label _label_5)
    (:`Update`
      (`CapsuleComponent.SetCapsuleHalfHeight` (`self.CapsuleComponent`) _half_height true))))

(event `CustomUnCrouch`
  ; Crouching
  (set `self.bCrouching` false)
  (set `CharacterMovementComponent.MaxWalkSpeed` 600.0 (`self.CharacterMovement`))
  (goto _label_5 :!via `Reverse`))

(event `EnhancedInput|/Game/FPSTest/Data/IA_Aim`
  (params (ActionValue :type Boolean) (ElapsedSeconds :type "Float (double-precision)") (TriggeredSeconds :type "Float (double-precision)") (InputAction :type "InputAction Object Reference" :default "/Game/FPSTest/Data/IA_Aim.IA_Aim"))
  ; Aim Bool
  (:`Triggered`
    (set `self.bAiming` true))
  (:`Completed`
    (set `self.bAiming` false)))

(event `self.ReceiveTick`
  (params (DeltaSeconds :type "Float (single-precision)"))
  (bind _camera (`self.Camera`))
  ; Rotation
  (`SceneComponent.K2_SetRelativeRotation` (`self.Pivot`) (`KismetMathLibrary.MakeRotator` 0.0 (.pitch (`self.GetControlRotation`))) false false)
  (bind (_outhit _returnvalue) (`KismetSystemLibrary.LineTraceSingle` (`SceneComponent.K2_GetComponentLocation` (`self.Camera`)) (+ (`SceneComponent.K2_GetComponentLocation` _camera) (* (`SceneComponent.GetForwardVector` _camera) (100.0 100.0 100.0))) "TraceTypeQuery1"))
  (set `self.bCloseToWall` _returnvalue))

(event `EnhancedInput|/Game/FPSTest/Data/IA_Shoot`
  (params (ActionValue :type Boolean) (ElapsedSeconds :type "Float (double-precision)") (TriggeredSeconds :type "Float (double-precision)") (InputAction :type "InputAction Object Reference" :default "/Game/FPSTest/Data/IA_Shoot.IA_Shoot"))
  ; Weapon Functionality
  (:`Triggered`
    (`/Engine/EditorBlueprintResources/StandardMacros.DoOnce` false :!label _label_6
      (:`Completed`
        (set `self.bHoldingShoot` true)
        (if (and (and (and (`self.bHoldingShoot`) (not (`self.bRunning`)) (not (`self.bCloseToWall`)) (> (`self.CurrentAmmunition`) 0)) (not (`self.bReloading`))) (`self.bEquipped`)) :!label _label_7
          (message `/Game/FPSTest/Core/BPI_Weapon.Shoot` (`|GetArrayItem` (`self.EquippedWeapons`) (`self.EquippedWeaponIndex`)))
          (`|PlayMontage` (`self.CharacterArms`) "/Game/FPSTest/Art/AssaultRifle/Animations/AM_FP_AssaultRifle_Fire_Montage.AM_FP_AssaultRifle_Fire_Montage"
            (:`then`
              (bind _returnvalue (`|SpawnActorFromClass` "/Game/FPSTest/Core/BP_Bullet.BP_Bullet_C" (`SceneComponent.K2_GetComponentToWorld` (`self.BulletEntry`)) "AlwaysSpawn" "MultiplyWithRoot" self self))
              (`PrimitiveComponent.IgnoreActorWhenMoving` (`/Game/FPSTest/Core/BP_Bullet.Sphere` _returnvalue) self true)
              (`PrimitiveComponent.IgnoreActorWhenMoving` (`self.CapsuleComponent`) _returnvalue false)
              (`GameplayStatics.SpawnEmitterAttached` "/Game/StarterContent/Particles/P_Explosion.P_Explosion" (`Actor.RootComponent` (`|GetArrayItem` (`self.EquippedWeapons`) (`self.EquippedWeaponIndex`))) "None" (0.0 60.0 0.0) (struct) (0.05 0.05 0.05) "SnapToTargetIncludingScale")
              (`KismetSystemLibrary.Delay` (`self.FireDelay`))
              (set `self.CurrentAmmunition` (- (`self.CurrentAmmunition`) 1))
              (goto _label_7)))))))
  (:`Completed`
    (set `self.bHoldingShoot` false)
    (goto _label_6 :!via `Reset`)))

(event `EnhancedInput|/Game/FPSTest/Data/IA_Reload`
  (params (ActionValue :type Boolean) (ElapsedSeconds :type "Float (double-precision)") (TriggeredSeconds :type "Float (double-precision)") (InputAction :type "InputAction Object Reference" :default "/Game/FPSTest/Data/IA_Reload.IA_Reload"))
  ; Reload
  (:`Triggered`
    (`/Engine/EditorBlueprintResources/StandardMacros.DoOnce` false :!label _label_8
      (:`Completed`
        (if (and (and (not (`self.bReloading`)) (< (`self.CurrentAmmunition`) (`self.MagSize`)) (> (`self.TotalAmmunition`) 0) (not (`self.bRunning`))) (`self.bEquipped`))
          (set `self.bReloading` true)
          (`|PlayMontage` (`self.CharacterArms`) "/Game/FPSTest/Art/AssaultRifle/Animations/AM_A_FP_AssaultRifle_Reload_Main.AM_A_FP_AssaultRifle_Reload_Main"
            (:`then`
              (set `self.bCanRun` false)
              (message `/Game/FPSTest/Core/BPI_Weapon.Reload` (`|GetArrayItem` (`self.EquippedWeapons`) (`self.EquippedWeaponIndex`))))
            (:`OnCompleted`
              (`KismetSystemLibrary.Delay` 0.0)
              (bind _output_get (set `self.MissingAmmo` (- (`self.MagSize`) (`self.CurrentAmmunition`))))
              (set `self.AmmoToReload` (`KismetMathLibrary.Min` _output_get (`self.TotalAmmunition`)))
              (set `self.CurrentAmmunition` (+ (`self.CurrentAmmunition`) (`self.AmmoToReload`)))
              (set `self.TotalAmmunition` (- (`self.TotalAmmunition`) (`self.AmmoToReload`)))
              (set `self.bReloading` false)
              (set `self.bCanRun` true)))))))
  (:`Completed`
    (goto _label_8 :!via `Reset`)))

(event `HolsterToggle`
  (if (not (`self.bReloading`)) :!label _label_9
    (set `self.bEquipped` (not (`self.bEquipped`)))
    (`|PlayMontage` (`self.CharacterArms`) (select `bool` (`self.bEquipped`) :`false` "/Game/FPSTest/Art/AssaultRifle/Animations/AM_FP_AssaultRifle_Holster.AM_FP_AssaultRifle_Holster" :`true` "/Game/FPSTest/Art/AssaultRifle/Animations/AM_FP_AssaultRifle_Equip.AM_FP_AssaultRifle_Equip" :!type "AnimMontage Object Reference"))))

(event `EnhancedInput|/Game/FPSTest/Data/IA_Holster`
  (params (ActionValue :type Boolean) (ElapsedSeconds :type "Float (double-precision)") (TriggeredSeconds :type "Float (double-precision)") (InputAction :type "InputAction Object Reference" :default "/Game/FPSTest/Data/IA_Holster.IA_Holster"))
  (:`Triggered`
    (`/Engine/EditorBlueprintResources/StandardMacros.DoOnce` false :!label _label_10
      (:`Completed`
        (goto _label_9))))
  (:`Completed`
    (goto _label_10 :!via `Reset`)))

(event `self.ReceiveAnyDamage`
  (params (Damage :type "Float (single-precision)") (DamageType :type "DamageType Object Reference") (InstigatedBy :type "Controller Object Reference") (DamageCauser :type "Actor Object Reference"))
  (bind _returnvalue (`GameplayStatics.GetPlayerController` 0))
  (bind _output_get (set `self.CurrentHealth` (- (`self.CurrentHealth`) Damage)))
  (`/Game/FPSTest/Core/WBP_PlayerUI.UpdateHealth` (`self.HealthUIRef`) _output_get (`self.MaxHealth`))
  (`KismetSystemLibrary.PrintString` (`KismetStringLibrary.Conv_DoubleToString` _output_get))
  (if (<= (`self.CurrentHealth`) 0.0)
    (bind _returnvalue_2 (`|CreateWidget` "/Game/UI/BP_EndScreen.BP_EndScreen_C"))
    (`UserWidget.AddToViewport` _returnvalue_2 0)
    (`WidgetBlueprintLibrary.SetInputMode_UIOnlyEx` _returnvalue null)
    (set `PlayerController.bShowMouseCursor` true _returnvalue)))

(fn `SpawnInventory`
  (for _array_element (`self.Inventory`)
    (bind _returnvalue (`|SpawnActorFromClass` _array_element (`KismetMathLibrary.MakeTransform` (0.0 0.0 0.0)) "Undefined" "MultiplyWithRoot" null null))
    (`KismetArrayLibrary.Array_Add` (`self.EquippedWeapons`) _returnvalue)
    (`self.K2_AttachToComponent` _returnvalue (`self.CharacterArms`) "ik_hand_gun" "KeepRelative" "KeepRelative" "KeepRelative" true)
    (`self.SetActorHiddenInGame` _returnvalue true))
  (`self.SetActorHiddenInGame` (`|GetArrayItem` (`self.EquippedWeapons`) (`self.EquippedWeaponIndex`)) false))

(fn `UserConstructionScript`)